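; BP_Packet visualizes a data packet travelling between a client and a peer, labelled on screen with its type.
; A pulsing timeline ping-pongs the mesh scale at a random rate from BeginPlay.
; OnSend picks the peer or client as destination based on the sender, then a randomly paced timeline lerps the mesh there.
; A viewport widget follows it via world-to-screen projection and is removed on completion, when Arrive is called.
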(event Custom|OnSendEvent
  (bind _data (Variables|Default|GetData))
  (bind (_client _peer _destinationpeer _type _sender) (Utilities|Struct|BreakPacketData _data))
  (bind _returnvalue (UserInterface|CreateWidget "/Game/UMG/UMG_PacketTypeText.UMG_PacketTypeText_C"))
  (bind _output_get (Variables|Default|SetPacketText _returnvalue))
  (UserInterface|Viewport|AddtoViewport _output_get 0)
  (if (Utilities|Enum|Equal(Enum) _sender "CLIENT")
    (Variables|Default|SetDestination (Transformation|GetActorLocation _destinationpeer))
    (else
      (Variables|Default|SetDestination (Transformation|GetActorLocation _client))))
  (Variables|Default|SetStartLocation (Transformation|GetWorldLocation (Variables|Default|GetStaticMeshComponent)))
  (Rendering|Components|TextRender|SetText (Variables|/Game/UMG/UMG_PacketTypeText.UMG_PacketTypeText_C|GetPacketTextBlock (Variables|Default|GetPacketText)) (Utilities|Text|ToText(String) _type))
  (bind _alpha (Timeline|Location Play)
    (:Update
      (Transformation|SetWorldLocation (Variables|Default|GetStaticMeshComponent) (Math|Vector|Lerp(Vector) (Variables|Default|GetStartLocation) (Variables|Default|GetDestination) _alpha) false false)
      (Class|UserWidget|SetPositioninViewport (Variables|Default|GetPacketText) (.ScreenPosition (Class|GameplayStatics|ProjectWorldtoScreen (Game|GetPlayerController 0) (Math|Vector|Lerp(Vector) (Variables|Default|GetStartLocation) (Variables|Default|GetDestination) _alpha))) true))
    (:Finished
      (Widget|RemovefromParent (Variables|Default|GetPacketText))
      (Class|Packet|Arrive))))

(event EventBeginPlay
  (Components|Timeline|SetPlayRate (Variables|Default|GetLocation) (Math|Random|RandomFloatinRange 0.4 1.2))
  (Components|Timeline|SetPlayRate (Variables|Default|GetPulsing) (Math|Random|RandomFloatinRange 0.5 1.0))
  (EventDispatchers|AssignOnSend (delegate Custom|OnSendEvent))
  ;[1 1 1] PulseForever
  (bind (_direction _scale) (Timeline|Pulsing Play)
    (:Update
      (Transformation|SetWorldScale3D (Variables|Default|GetStaticMeshComponent) (Math|Conversions|ToVector(Float) _scale)))
    (:Finished
      (Utilities|FlowControl|RetriggerableDelay 0.02)
      (if (Utilities|Enum|Equal(Enum) _direction "Forward")
        (Timeline|Pulsing Reverse)
        (else
          (Timeline|Pulsing Play))))))

(fn ConstructionScript)