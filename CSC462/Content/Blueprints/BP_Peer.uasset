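; BP_Peer is a clickable peer node whose active state toggles on each click, with its mesh color showing the state.
; BeginPlay creates a dynamic instance of M_Peers on the static mesh and caches its original Color parameter.
; Clicking the mesh flips IsActive, painting it red when deactivated and restoring the cached color when reactivated.
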(event OnClicked(StaticMeshComponent)
  (params (TouchedComponent :type Primitive%20Component%20Object%20Reference) (ButtonPressed :type Key%20Structure :default "AnyKey"))
  (bind _materialinstance (Variables|Default|GetMaterialInstance))
  ;[1 1 1] Toggle whether the node is active or not
  (if (Variables|Default|GetbIsActive)
    (Rendering|Material|SetVectorParameterValue _materialinstance "Color" "(R=0.920000,G=0.046000,B=0.046000,A=1.000000)" :!class /Script/Engine.MaterialInstanceDynamic)
    (else
      (Rendering|Material|SetVectorParameterValue _materialinstance "Color" (Variables|Default|GetOriginalColor) :!class /Script/Engine.MaterialInstanceDynamic)))
  (Variables|Default|SetbIsActive (not (Variables|Default|GetbIsActive))))

(event EventBeginPlay
  ;[1 1 1] Get material instance
  (bind _returnvalue (Rendering|Material|CreateDynamicMaterialInstance (Variables|Default|GetStaticMeshComponent) 0 "/Game/Materials/M_Peers.M_Peers" :!class /Script/Engine.PrimitiveComponent))
  (bind _output_get (Variables|Default|SetMaterialInstance _returnvalue))
  (bind _returnvalue_2 (Rendering|Material|GetVectorParameterValue _output_get "Color" :!class /Script/Engine.MaterialInstanceDynamic))
  (Variables|Default|SetOriginalColor _returnvalue_2))

(fn ConstructionScript)